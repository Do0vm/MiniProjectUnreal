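; BP_Rifle is a rifle that fires BP_Bullet actors when its ShootingEvent is called.
; Each shot spawns a bullet at the Scene component's transform, taking only its yaw with a slight random spread, so pitch and roll are not carried over.
; It then activates the Niagara muzzle flash, plays a 2D shot sound and switches the flash off after a short delay, sharing that deactivation with BeginPlay.
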(event `self.ReceiveBeginPlay`
  (`ActorComponent.Deactivate` (`self.NS_MuzzleFlash`) :!label _label))

(event `ShootingEvent`
  (bind _returnvalue (`SceneComponent.K2_GetComponentToWorld` (`self.Scene`)))
  ;[0 0.08333 0.05387] BulletSpawning
  (`|SpawnActorFromClass` "/Game/MillAssets/Gun/BP_Bullet.BP_Bullet_C" (`KismetMathLibrary.MakeTransform` (.location _returnvalue) (`KismetMathLibrary.MakeRotator` 0.0 0.0 (`KismetMathLibrary.RandomFloatInRange` (- (.yaw (.rotation _returnvalue)) 0.1) (+ (.yaw (.rotation _returnvalue)) 0.1))) (.scale _returnvalue)) "Undefined" "MultiplyWithRoot" null null)
  (`ActorComponent.Activate` (`self.NS_MuzzleFlash`) true)
  (`GameplayStatics.PlaySound2D` "/Game/Sound/Guns/Rifle/RigleShot.RigleShot" 1.0 1.0 0.0 null null)
  (`KismetSystemLibrary.Delay` 0.1)
  (goto _label))

(fn `UserConstructionScript`)