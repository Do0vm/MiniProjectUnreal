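; Exploding zombie enemy that roams the navmesh and chases the top-down player character on sight.
; A delayed AIMoveTo loop picks random reachable points; pawn sensing switches to chasing with a sound, and roaming is re-triggered after the chase move completes.
; Hitting the seen player deals damage with explosion effects and force feedback, then ragdolls and destroys the zombie.
; Incoming damage triggers blood; at zero health it ragdolls with an impulse, then removes its mesh.
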(event `self.ReceiveAnyDamage`
  (params (Damage :type "Float (single-precision)") (DamageType :type "DamageType Object Reference") (InstigatedBy :type "Controller Object Reference") (DamageCauser :type "Actor Object Reference"))
  (bind _mesh (`self.Mesh`))
  (bind (_returnvalue_x _returnvalue_y) (`KismetMathLibrary.BreakVector` (* (`self.GetActorForwardVector` DamageCauser) 5000.0)))
  (bind _output_get (set `self.Health` (- (`self.Health`) Damage)))
  (`ActorComponent.Activate` (`self.NS_OmniBlood`) true)
  (if (<= _output_get 0.0)
    (`PrimitiveComponent.SetCollisionProfileName` _mesh "Ragdoll" true)
    (`PrimitiveComponent.SetSimulatePhysics` _mesh true)
    (`PrimitiveComponent.AddImpulse` _mesh (`KismetMathLibrary.MakeVector` _returnvalue_x _returnvalue_y) "None" true)
    (`ActorComponent.K2_DestroyComponent` (`self.CapsuleComponent`))
    (`KismetSystemLibrary.Delay` 3.0)
    (`ActorComponent.K2_DestroyComponent` (`self.Mesh`))))

(event `RoamingMapAI`
  (bind _randomlocation (`NavigationSystemV1.K2_GetRandomLocationInNavigableRadius` (`self.K2_GetActorLocation`) (`self.Radius`) null null :!label _label))
  (`|AIMoveTo` self _randomlocation null
    (:`then`
      (`KismetSystemLibrary.PrintString` "AI is roamin" true true (struct :`G` 1.0 :`B` 0.78562 :`A` 1.0)))
    (:`OnFail`
      (`KismetSystemLibrary.PrintString` "AI is not romaing" true true (struct :`R` 0.767893 :`B` 1.0 :`A` 1.0))))
  (`KismetSystemLibrary.Delay` (`self.Duration`))
  (if (not (`self.CanSeePlayer`))
    (goto _label)))

(event `self.ReceiveBeginPlay`
  (bind _asbp_top_down_character (cast `/Game/TopDown/Blueprints/BP_TopDownCharacter` (`GameplayStatics.GetPlayerCharacter` 0)))
  (set `self.As BP Top Down Character` _asbp_top_down_character)
  (goto _label))

(event `self.CapsuleComponent.OnComponentHit`
  (params (HitComponent :type "PrimitiveComponent Object Reference") (OtherActor :type "Actor Object Reference") (OtherComp :type "PrimitiveComponent Object Reference") (NormalImpulse :type "Vector Structure") (Hit :type "HitResult Structure (by ref)"))
  (bind _mesh (`self.Mesh`))
  (bind _as_bp_top_down_character (`self.As BP Top Down Character`))
  (bind (_returnvalue_x _returnvalue_y) (`KismetMathLibrary.BreakVector` (* (`self.GetActorForwardVector`) 5000.0)))
  (if (== OtherActor _as_bp_top_down_character)
    (if (`self.CanSeePlayer`)
      (`GameplayStatics.ApplyDamage` _as_bp_top_down_character 2.0 null self)
      (`GameplayStatics.SpawnEmitterAtLocation` "/Game/StarterContent/Particles/P_Explosion.P_Explosion" (`self.K2_GetActorLocation`))
      (`GameplayStatics.PlaySoundAtLocation` "/Game/StarterContent/Audio/Explosion01.Explosion01" (`self.K2_GetActorLocation`) (struct) 1.0 1.0 0.0 null null null null)
      (`PlayerController.K2_ClientPlayForceFeedback` (`GameplayStatics.GetPlayerController` 0) "/Game/TopDown/Input/ExplosiveFeedback.ExplosiveFeedback" "None" false false false)
      (`PrimitiveComponent.SetCollisionProfileName` _mesh "Ragdoll" true)
      (`PrimitiveComponent.SetSimulatePhysics` _mesh true)
      (`PrimitiveComponent.AddImpulse` _mesh (`KismetMathLibrary.MakeVector` _returnvalue_x _returnvalue_y) "None" true)
      (`ActorComponent.K2_DestroyComponent` (`self.CapsuleComponent`))
      (`KismetSystemLibrary.Delay` 4.0)
      (`self.K2_DestroyActor`))))

(event `self.ZombieSensing.OnSeePawn`
  (params (Pawn :type "Pawn Object Reference"))
  (if (== Pawn (`self.As BP Top Down Character`))
    (set `self.CanSeePlayer` true)
    (`|ExecutionSequence`
      (:`then_0`
        (`|AIMoveTo` self (0.0 0.0 0.0) (`self.As BP Top Down Character`)
          (:`then`
            (`KismetSystemLibrary.PrintString` "Ai is Not lost" true true (struct :`R` 0.406678 :`G` 1.0 :`A` 1.0))
            (`KismetSystemLibrary.RetriggerableDelay` 3.0)
            (`self.RoamingMapAI`))
          (:`OnFail`
            (`KismetSystemLibrary.PrintString` "Ai is lost" true true (struct :`R` 1.0 :`B` 0.842126 :`A` 1.0)))))
      (:`then_1`
        (`/Engine/EditorBlueprintResources/StandardMacros.DoOnce` false
          (:`Completed`
            (`GameplayStatics.PlaySoundAtLocation` (`self.Chase`) (`self.K2_GetActorLocation`) (struct) 1.0 1.0 0.0 null null null null)))))
    (else
      (set `self.CanSeePlayer` false))))

(fn `UserConstructionScript`)